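; Item spawner actor that keeps a randomized BP_Item (fruit) available at its location.
; SpawnFruit runs at BeginPlay, spawning the item at the spawner's transform, randomizing it and storing it as SpawnedItem.
; Tick releases the tracked item and spawns another once it is 500 units or more away, or whenever the reference is invalid.
; An OnDestroyed handler for SpawnedItem also triggers a respawn.
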(event OnDestroyed(SpawnedItem)
  (params (DestroyedActor :type Actor%20Object%20Reference))
  (CallFunction|SpawnFruit))

(event Custom|SpawnFruit
  (bind _returnvalue (Game|SpawnActorfromClass "/Game/Blueprints/BP_Item.BP_Item_C" (Transformation|GetActorTransform) "Undefined" 0 0))
  (Default|RandomizeItem _returnvalue)
  (Variables|Default|SetSpawnedItem _returnvalue))

(event EventBeginPlay
  (CallFunction|SpawnFruit))

(event Collision|EventActorBeginOverlap
  (params (OtherActor :type Actor%20Object%20Reference)))

(event EventTick
  (params (DeltaSeconds :type Float%20%28single-precision%29))
  (Utilities|IsValid (Variables|Default|GetSpawnedItem)
    (:Is%20Valid
      (if (>= (Transformation|GetDistanceTo (Variables|Default|GetSpawnedItem) self) 5e+02)
        (Variables|Default|SetSpawnedItem 0)
        (CallFunction|SpawnFruit)))
    (:Is%20Not%20Valid
      (CallFunction|SpawnFruit))))

(fn ConstructionScript)