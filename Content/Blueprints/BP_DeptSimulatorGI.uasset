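; Game Instance for a debt simulator that tracks cash and debt over time and shows a loss screen when cash runs out.
; On Init it adds the overlay widget after a short delay and starts a looping timer.
; Each tick counts the interval, subtracts the loan installment from debt, adds NPC payments minus that installment to cash, updates the overlay, then checks for loss.
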(event EventInit
  (Utilities|FlowControl|Sequence
    (:then_0
      ;[1 1 1] Add Overlay to Viewport
      (Utilities|FlowControl|Delay 0.1)
      (bind _returnvalue (UserInterface|CreateWidget "/Game/UI/W_Overlay.W_Overlay_C" (Game|GetPlayerController 0)))
      (bind _output_get (Variables|Default|SetW_Overlay _returnvalue))
      (UserInterface|Viewport|AddtoViewport _output_get 0))
    (:then_1
      ;[1 1 1] TracksTime
      (Utilities|Time|SetTimerbyFunctionName 0 "TimeIncrementEvent" (Variables|Default|GetTimeIntervalSeconds) true))))

(fn TimeIncrementEvent
  (Math|Integer|IncrementInt (Variables|Default|GetNumberOfTimeIncrementsPassed)
    (:%20%20
      (Variables|Default|SetTotalDebt (- (Variables|Default|GetTotalDebt) (Variables|Default|GetLoanInstallmentInterval)))
      (Variables|Default|SetTotalCash (+ (Variables|Default|GetTotalCash) (- (Variables|Default|GetTotalNPCPaymentInterval) (Variables|Default|GetLoanInstallmentInterval))))
      (Default|TimeIncrement (Variables|Default|GetW_Overlay))
      (if (<= (Variables|Default|GetTotalCash) 0)
        (bind _returnvalue (UserInterface|CreateWidget "/Game/UI/W_Lost.W_Lost_C"))
        (UserInterface|Viewport|AddtoViewport _returnvalue 0)))))